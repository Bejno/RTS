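; RTS-style HUD that provides screen-edge camera scrolling and drag-box unit selection, with the mouse locked to the screen.
; DrawHUD builds eight edge hitboxes whose comma-encoded names are parsed on hover to set EdgeScrollingPawn's movement axes, except during selection.
; It also draws the selection box and updates SelectedActorsList in replace, Shift-add or Ctrl-remove mode, toggling selection on SquareUnits.
; MoveActor sends selected units to the world origin.
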(event Custom|StopShiftSelectionBox
  (Variables|Default|SetDrawShiftSelectionBox? false)
  (Utilities|Array|Clear (Variables|Default|GetTempSelectedActorsList)))

(event Custom|CtrlSelectionBox
  (params (FirstMousePosition :type Vector%202D%20Structure))
  (Variables|Default|SetFirstMousePosition FirstMousePosition)
  (Variables|Default|SetDrawRegulareSelectionBox? false)
  (Variables|Default|SetDrawShiftSelectionBox? false)
  (Variables|Default|SetDrawCtrlSelectionBox? true))

(event Custom|StopCtrlSelectionBox
  (Variables|Default|SetDrawCtrlSelectionBox? false)
  (Utilities|Array|Clear (Variables|Default|GetTempSelectedActorsList)))

(event Custom|MoveActor
  (for _array_element (Variables|Default|GetSelectedActorsList)
    (bind _assquare_unit (Utilities|Casting|CastToSquareUnit _array_element))
    (Default|MovetoLocation _assquare_unit "0, 0, 0")))

(event Custom|RegulareSelectionBox
  (params (FirstMousePosition :type Vector%202D%20Structure))
  (bind _selectedactorslist (Variables|Default|GetSelectedActorsList))
  (Variables|Default|SetFirstMousePosition FirstMousePosition)
  (Variables|Default|SetDrawRegulareSelectionBox? true)
  (Variables|Default|SetDrawShiftSelectionBox? false)
  (Variables|Default|SetDrawCtrlSelectionBox? false)
  (for _array_element _selectedactorslist
    (CallFunction|SelectUnits true _array_element))
  (Utilities|Array|Clear _selectedactorslist))

(event Custom|StopRegulareSelectionBox
  (Variables|Default|SetDrawRegulareSelectionBox? false)
  (Utilities|Array|Clear (Variables|Default|GetTempSelectedActorsList)))

(event Custom|ShiftSelectionBox
  (params (FirstMousePosition :type Vector%202D%20Structure))
  (Variables|Default|SetFirstMousePosition FirstMousePosition)
  (Variables|Default|SetDrawRegulareSelectionBox? false)
  (Variables|Default|SetDrawShiftSelectionBox? true)
  (Variables|Default|SetDrawCtrlSelectionBox? false))

(event EventHitBoxBeginCursorOver
  (params (BoxName :type Name))
  ;[1 1 1] Detect Mouse Over/Mouse Leave Hitbox and move the camera if not drawing selection box
  (if (not (Math|Boolean|ORBoolean (Variables|Default|GetDrawRegulareSelectionBox?) (Variables|Default|GetDrawShiftSelectionBox?) (Variables|Default|GetDrawCtrlSelectionBox?)))
    (bind _element_id_s (Utilities|GetHitboxType BoxName)
      (:EdgeBox
        (Utilities|EdgeBoxEvents _element_id_s
          (:Top%20Left
            (Utilities|EdgeMovmement :!label _label))
          (:TopMiddle
            (goto _label TopMiddle))
          (:TopRight
            (goto _label TopRight))
          (:MiddleRight
            (goto _label MiddleRight))
          (:BottomRight
            (goto _label BottomRight))
          (:BottomMiddle
            (goto _label BottomMiddle))
          (:BottomLeft
            (goto _label BottomLeft))
          (:MiddleLeft
            (goto _label MiddleLeft)))))))

(event EventHitBoxEndCursorOver
  (params (BoxName :type Name))
  ;[1 1 1] Detect Mouse Over/Mouse Leave Hitbox and move the camera if not drawing selection box
  (bind _element_id_s (Utilities|GetHitboxType BoxName)
    (:EdgeBox
      (Utilities|EdgeBoxEvents _element_id_s
        (:Top%20Left
          _)
        (:TopMiddle
          _)
        (:TopRight
          _)
        (:MiddleRight
          _)
        (:BottomRight
          _)
        (:BottomMiddle
          _)
        (:BottomLeft
          _)
        (:MiddleLeft
          _))
      (CallFunction|ResetEdgeMovement))))

(event EventBeginPlay
  ;[1 1 1] Lock Mouse to screen
  (bind _asedge_scrolling_pawn (Utilities|Casting|CastToEdgeScrollingPawn (Class|HUD|GetOwningPawn)))
  (Variables|Default|SetOwningPawn _asedge_scrolling_pawn)
  (Input|SetInputModeGameandUI (Game|GetPlayerController 0) 0 "LockAlways" false))

(event EventDrawHUD
  (params (SizeX :type Integer) (SizeY :type Integer))
  (bind _returnvalue (Game|GetPlayerController 0))
  (bind _firstmouseposition (Variables|Default|GetFirstMousePosition))
  (bind (_locationx _locationy) (Game|Player|GetMousePosition _returnvalue))
  (bind _returnvalue_2 (Math|Vector2D|MakeVector2D _locationx _locationy))
  (bind _outactors (Class|HUD|GetActorsinSelectionRectangle "/Game/OwnContent/Blueprints/Units/UnitParent.UnitParent_C" _firstmouseposition _returnvalue_2 false false))
  (Utilities|FlowControl|Sequence
    (:then_0
      ;[1 1 1] Draw Edge Hitbox
      (Variables|Default|SetScreenRes (Math|Vector2D|MakeVector2D (Math|Conversions|ToFloat(Integer) SizeX) (Math|Conversions|ToFloat(Integer) SizeY)))
      (CallFunction|DrawEdgeHitboxes :Size (Variables|Default|GetScreenRes) :EdgeThickness 32.0 :bShowOverlays? true :OverlayColour "(R=0.307248,G=0.850000,B=0.165750,A=1.000000)" :bConsumeInput? true))
    (:then_1
      (if (Variables|Default|GetDrawRegulareSelectionBox?)
        (CallFunction|DrawSelectionBoxGrafic)
        (bind _output_get (Variables|Default|SetTempSelectedActorsList _outactors))
        (for _array_element _output_get
          (Utilities|Array|Add (Variables|Default|GetSelectedActorsList) _array_element)
          (CallFunction|SelectUnits false _array_element))
        (bind _outactors_2 (Actor|GetAllActorswithTag "Friendly"))
        (for _array_element_2 _outactors_2
          (if (Utilities|Array|ContainsItem (Variables|Default|GetSelectedActorsList) _array_element_2)
            (if (not (Utilities|Array|ContainsItem (Variables|Default|GetTempSelectedActorsList) _array_element_2))
              (CallFunction|SelectUnits true _array_element_2)
              (Utilities|Array|RemoveItem (Variables|Default|GetSelectedActorsList) _array_element_2))))
        (elif (Variables|Default|GetDrawShiftSelectionBox?)
          (CallFunction|DrawSelectionBoxGrafic)
          (bind _output_get_2 (Variables|Default|SetTempSelectedActorsList _outactors))
          (for _array_element_3 _output_get_2
            (if (not (Utilities|Array|ContainsItem (Variables|Default|GetSelectedActorsList) _array_element_3))
              (Utilities|Array|Add (Variables|Default|GetSelectedActorsList) _array_element_3)
              (CallFunction|SelectUnits false _array_element_3)))
          (elif (Variables|Default|GetDrawCtrlSelectionBox?)
            (CallFunction|DrawSelectionBoxGrafic)
            (Variables|Default|SetTempSelectedActorsList _outactors)
            (for _array_element_4 _outactors
              (if (Utilities|Array|ContainsItem (Variables|Default|GetSelectedActorsList) _array_element_4)
                (CallFunction|SelectUnits true _array_element_4)
                (Utilities|Array|RemoveItem (Variables|Default|GetSelectedActorsList) _array_element_4)))))))))

(fn ConstructionScript)

(fn DrawHitBoxwithOverlay
  (params (Position :type Vector%202D%20Structure) (Size :type Vector%202D%20Structure) (Name :type Name) (bConsumeInput? :type Boolean) (Priority :type Integer) (bShowOverlay? :type Boolean) (OverlayColour :type Linear%20Color%20Structure))
  (bind (_x _y) (Math|Vector2D|BreakVector2D Size))
  (bind (_x_2 _y_2) (Math|Vector2D|BreakVector2D Position))
  (Class|HUD|AddHitBox Position Size Name bConsumeInput? Priority)
  (if bShowOverlay?
    (HUD|DrawRect OverlayColour _x_2 _y_2 _x _y)))

(fn DrawEdgeHitboxes
  (params (ID :type Integer) (Location :type Vector%202D%20Structure) (Size :type Vector%202D%20Structure) (EdgeThickness :type Float%20%28single-precision%29) (bShowOverlays? :type Boolean) (OverlayColour :type Linear%20Color%20Structure) (bConsumeInput? :type Boolean) (Priority :type Integer))
  (LocalVariables|SetIdL ID)
  (LocalVariables|SetLocationL Location)
  (LocalVariables|SetSizeL Size)
  (LocalVariables|SetEdgeThicknessL EdgeThickness)
  (LocalVariables|SetShowOverlaysL bShowOverlays?)
  (LocalVariables|SetOverlayColourL OverlayColour)
  (LocalVariables|SetConsumeInputL bConsumeInput?)
  (LocalVariables|SetPriorityL Priority)
  (for _index (range 0 7)
    (CallFunction|DrawHitBoxwithOverlay (Utilities|Select :Index _index :Option%200 (.Top%20Left (Utilities|GetLocationforEdges (LocalVariables|GetLocationL) (LocalVariables|GetSizeL) (LocalVariables|GetEdgeThicknessL))) :Option%201 (.Top%20Middle (Utilities|GetLocationforEdges (LocalVariables|GetLocationL) (LocalVariables|GetSizeL) (LocalVariables|GetEdgeThicknessL))) :Option%202 (.Top%20Right (Utilities|GetLocationforEdges (LocalVariables|GetLocationL) (LocalVariables|GetSizeL) (LocalVariables|GetEdgeThicknessL))) :Option%203 (.Middle%20Right (Utilities|GetLocationforEdges (LocalVariables|GetLocationL) (LocalVariables|GetSizeL) (LocalVariables|GetEdgeThicknessL))) :Option%204 (.Bottom%20Right (Utilities|GetLocationforEdges (LocalVariables|GetLocationL) (LocalVariables|GetSizeL) (LocalVariables|GetEdgeThicknessL))) :Option%205 (.Bottom%20Middle (Utilities|GetLocationforEdges (LocalVariables|GetLocationL) (LocalVariables|GetSizeL) (LocalVariables|GetEdgeThicknessL))) :Option%206 (.Bottom%20Left (Utilities|GetLocationforEdges (LocalVariables|GetLocationL) (LocalVariables|GetSizeL) (LocalVariables|GetEdgeThicknessL))) :Option%207 (.Middle%20Left (Utilities|GetLocationforEdges (LocalVariables|GetLocationL) (LocalVariables|GetSizeL) (LocalVariables|GetEdgeThicknessL)))) (Utilities|Select :Index _index :Option%200 (Math|Vector2D|MakeVector2D (LocalVariables|GetEdgeThicknessL) (LocalVariables|GetEdgeThicknessL)) :Option%201 (.XLength (Utilities|CreateEdgeHitboxSize (LocalVariables|GetSizeL) (LocalVariables|GetEdgeThicknessL))) :Option%202 (Math|Vector2D|MakeVector2D (LocalVariables|GetEdgeThicknessL) (LocalVariables|GetEdgeThicknessL)) :Option%203 (.YLength (Utilities|CreateEdgeHitboxSize (LocalVariables|GetSizeL) (LocalVariables|GetEdgeThicknessL))) :Option%204 (Math|Vector2D|MakeVector2D (LocalVariables|GetEdgeThicknessL) (LocalVariables|GetEdgeThicknessL)) :Option%205 (.XLength (Utilities|CreateEdgeHitboxSize (LocalVariables|GetSizeL) (LocalVariables|GetEdgeThicknessL))) :Option%206 (Math|Vector2D|MakeVector2D (LocalVariables|GetEdgeThicknessL) (LocalVariables|GetEdgeThicknessL)) :Option%207 (.YLength (Utilities|CreateEdgeHitboxSize (LocalVariables|GetSizeL) (LocalVariables|GetEdgeThicknessL)))) (Utilities|CreateHitboxName "EdgeBox" (LocalVariables|GetIdL) _index) (LocalVariables|GetConsumeInputL) (LocalVariables|GetPriorityL) (LocalVariables|GetShowOverlaysL) (LocalVariables|GetOverlayColourL))))

(fn ResetEdgeMovement
  (bind _owningpawn (Variables|Default|GetOwningPawn))
  (Variables|/Game/OwnContent/Blueprints/EdgeScrollingPawn.EdgeScrollingPawn_C|SetEdgeForwardAxis _owningpawn 0.0)
  (Variables|/Game/OwnContent/Blueprints/EdgeScrollingPawn.EdgeScrollingPawn_C|SetEdgeRightAxis _owningpawn 0.0))

(fn SelectUnits
  (params (DeselectUnits? :type Boolean) (Actor :type Actor%20Object%20Reference))
  (LocalVariables|SetCurrentActor Actor)
  (LocalVariables|SetbDeselectUnits? DeselectUnits?)
  (bind _assquare_unit (Utilities|Casting|CastToSquareUnit (LocalVariables|GetCurrentActor)))
  (if (LocalVariables|GetbDeselectUnits?)
    (Default|Deselected _assquare_unit)
    (else
      (Default|Selected _assquare_unit))))

(fn DrawSelectionBoxGrafic
  (bind _returnvalue (Game|GetPlayerController 0))
  (bind _firstmouseposition (Variables|Default|GetFirstMousePosition))
  (bind _firstmouseposition_2 (Variables|Default|GetFirstMousePosition))
  (bind _firstmouseposition_3 (Variables|Default|GetFirstMousePosition))
  (bind (_x _y) (Math|Vector2D|BreakVector2D _firstmouseposition))
  (bind (_locationx _locationy) (Game|Player|GetMousePosition _returnvalue))
  (bind (_x_2 _y_2) (Math|Vector2D|BreakVector2D _firstmouseposition_2))
  (bind (_x_3 _y_3) (Math|Vector2D|BreakVector2D _firstmouseposition_3))
  (LocalVariables|SetMousePosition (Math|Vector2D|MakeVector2D _locationx _locationy)) ; Set current mouse position
  ;[1 1 1] Draw selection box square
  (HUD|DrawRect "(R=0.006557,G=0.135078,B=0.860000,A=0.500000)" _x _y (- (.X (Math|Vector2D|BreakVector2D (LocalVariables|GetMousePosition))) _x) (- (.Y (Math|Vector2D|BreakVector2D (LocalVariables|GetMousePosition))) _y))
  ;[1 1 1] Draw selection box line from (X¹,Y¹) to (X²,Y¹)
  (Class|HUD|DrawLine _x_2 _y_2 (.X (Math|Vector2D|BreakVector2D (LocalVariables|GetMousePosition))) _y_2 (LocalVariables|GetLineColor) (LocalVariables|GetLineTickness))
  ;[1 1 1] Draw selection box line from (X¹,Y¹) to (X¹,Y²)
  (Class|HUD|DrawLine _x_3 _y_3 _x_3 (.Y (Math|Vector2D|BreakVector2D (LocalVariables|GetMousePosition))) (LocalVariables|GetLineColor) (LocalVariables|GetLineTickness))
  ;[1 1 1] Draw selection box line from (X²,Y²) to (X¹,Y²)
  (Class|HUD|DrawLine (.X (Math|Vector2D|BreakVector2D (LocalVariables|GetMousePosition))) (.Y (Math|Vector2D|BreakVector2D (LocalVariables|GetMousePosition))) (.X (Math|Vector2D|BreakVector2D (LocalVariables|GetMousePosition))) (.Y (Math|Vector2D|BreakVector2D (Variables|Default|GetFirstMousePosition))) (LocalVariables|GetLineColor) (LocalVariables|GetLineTickness))
  ;[1 1 1] Draw selection box line from (X²,Y²) to (X²,Y¹)
  (Class|HUD|DrawLine (.X (Math|Vector2D|BreakVector2D (LocalVariables|GetMousePosition))) (.Y (Math|Vector2D|BreakVector2D (LocalVariables|GetMousePosition))) (.X (Math|Vector2D|BreakVector2D (Variables|Default|GetFirstMousePosition))) (.Y (Math|Vector2D|BreakVector2D (LocalVariables|GetMousePosition))) (LocalVariables|GetLineColor) (LocalVariables|GetLineTickness)))