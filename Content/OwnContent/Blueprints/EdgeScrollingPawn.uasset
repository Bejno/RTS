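; RTS-style camera pawn that pans, zooms and forwards selection and move-order input to EdgeScrollingHUD.
; Movement adds EdgeForwardAxis and EdgeRightAxis to input axes, relative to camera yaw.
; The camera sits on a sphere around the pawn, looking at its center, with mouse-wheel-controlled radius.
; LMB, Shift and Ctrl variants drive selection boxes, right-click calls MoveActor; rotation toggles and pitch logic are disconnected.
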(event EventBeginPlay
  (bind _returnvalue (Game|GetPlayerController 0))
  (Variables|Default|SetCameraComponent (Variables|Default|GetCamera))
  (Utilities|Casting|CastToEdgeScrollingPC _returnvalue)
  (bind _asedge_scrolling_hud (Utilities|Casting|CastToEdgeScrollingHUD (HUD|GetHUD _returnvalue))))

(event Input|ActionEvents|InputActionWheelMouseUp
  (params (Key :type Key%20Structure :default "AnyKey"))
  ;[1 1 1] Camera Zoom
  (:Pressed
    (Variables|Default|SetCameraRadius (Math|Float|Clamp(Float) (- (Variables|Default|GetCameraRadius) (Variables|Default|GetZoomSpeed)) (Variables|Default|GetRadiusMin) (Variables|Default|GetRadiusMax)))
    (CallFunction|UpdateCameraLocation&Rotation)))

(event Input|ActionEvents|InputActionWheelMouseDown
  (params (Key :type Key%20Structure :default "AnyKey"))
  ;[1 1 1] Camera Zoom
  (:Pressed
    (Variables|Default|SetCameraRadius (Math|Float|Clamp(Float) (+ (Variables|Default|GetCameraRadius) (Variables|Default|GetZoomSpeed)) (Variables|Default|GetRadiusMin) (Variables|Default|GetRadiusMax)))
    (CallFunction|UpdateCameraLocation&Rotation)))

(event Input|ActionEvents|InputActionLMB
  (params (Key :type Key%20Structure :default "AnyKey"))
  (bind _returnvalue (Game|GetPlayerController 0))
  (bind (_locationx _locationy) (Game|Player|GetMousePosition _returnvalue))
  (:Pressed
    (Default|RegulareSelectionBox (stale EventBeginPlay _asedge_scrolling_hud) (Math|Vector2D|MakeVector2D _locationx _locationy)))
  (:Released
    (Default|StopRegulareSelectionBox (stale EventBeginPlay _asedge_scrolling_hud))))

(event Input|ActionEvents|InputActionShiftLMB
  (params (Key :type Key%20Structure :default "AnyKey"))
  (bind _returnvalue (Game|GetPlayerController 0))
  (bind (_locationx _locationy) (Game|Player|GetMousePosition _returnvalue))
  (:Pressed
    (Default|ShiftSelectionBox (stale EventBeginPlay _asedge_scrolling_hud) (Math|Vector2D|MakeVector2D _locationx _locationy)))
  (:Released
    (Default|StopShiftSelectionBox (stale EventBeginPlay _asedge_scrolling_hud))))

(event Input|ActionEvents|InputActionCtrlLMB
  (params (Key :type Key%20Structure :default "AnyKey"))
  (bind _returnvalue (Game|GetPlayerController 0))
  (bind (_locationx _locationy) (Game|Player|GetMousePosition _returnvalue))
  (:Pressed
    (Default|CtrlSelectionBox (stale EventBeginPlay _asedge_scrolling_hud) (Math|Vector2D|MakeVector2D _locationx _locationy)))
  (:Released
    (Default|StopCtrlSelectionBox (stale EventBeginPlay _asedge_scrolling_hud))))

(event Input|ActionEvents|InputActionRotateCamera
  (params (Key :type Key%20Structure :default "AnyKey"))
  ;[1 1 1] Camera Rotation
)

(event Input|AxisEvents|InputAxisMouseX
  (params (AxisValue :type Float%20%28single-precision%29))
  ;[1 1 1] Camera Rotation
  (if (Variables|Default|GetbRotateCamera?)
    (Variables|Default|SetCameraZAngle (+ (* AxisValue (Variables|Default|GetRotateSpeed)) (Variables|Default|GetCameraZAngle)))
    (CallFunction|UpdateCameraLocation&Rotation)))

(event Input|AxisEvents|InputAxisMoveForward
  (params (AxisValue :type Float%20%28single-precision%29))
  ;[1 1 1] Camera Movment
  (Transformation|SetActorLocation (Utilities|AddVectortoLocation (Math|Vector|GetForwardVector (Utilities|IsloateYaw (Transformation|GetWorldRotation (Variables|Default|GetCamera)))) (* (+ AxisValue (Variables|Default|GetEdgeForwardAxis)) (Variables|Default|GetMovementSpeed))) false false))

(event Input|AxisEvents|InputAxisMouseY
  (params (AxisValue :type Float%20%28single-precision%29))
  ;[1 1 1] Camera Rotation
)

(event Input|AxisEvents|InputAxisMoveRight
  (params (AxisValue :type Float%20%28single-precision%29))
  ;[1 1 1] Camera Movment
  (Transformation|SetActorLocation (Utilities|AddVectortoLocation (Math|Vector|GetRightVector (Utilities|IsloateYaw (Transformation|GetWorldRotation (Variables|Default|GetCamera)))) (* (+ AxisValue (Variables|Default|GetEdgeRightAxis)) (Variables|Default|GetMovementSpeed))) false false))

(event Input|MouseEvents|RightMouseButton
  (params (Key :type Key%20Structure :default "AnyKey"))
  (:Pressed
    (Default|MoveActor (stale EventBeginPlay _asedge_scrolling_hud))))

(fn ConstructionScript
  (CallFunction|UpdateCameraLocation&Rotation))

(fn UpdateCameraLocation&Rotation
  (bind _camera (Variables|Default|GetCamera))
  (Transformation|SetRelativeLocation _camera (.Location (Utilities|PointonASphere (Variables|Default|GetCameraRadius) (Variables|Default|GetCameraZAngle) (Variables|Default|GetCameraHeightAngle))) false false)
  (Transformation|SetRelativeRotation _camera (Math|Rotator|FindLookatRotation (Variables|/Script/Engine.SceneComponent|GetRelativeLocation (Variables|Default|GetCamera)) (Math|Vector|MakeVector 0.0 0.0 0.0)) false false))